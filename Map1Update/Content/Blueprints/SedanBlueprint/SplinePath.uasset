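; Spline path actor that holds world-space points, per-point steering suggestions and forward/back connections, apparently for vehicle path following.
; The Construction Script applies the closed-loop setting, resizes the suggestion array to match the point count and caches point locations as transforms.
; It can optionally label each point with its index using text render components.
; Getter functions expose the connections, transforms and suggestion data.
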(event EventBeginPlay)

(event EventActorBeginOverlap
  (params (OtherActor :type Actor%20Object%20Reference)))

(event EventTick
  (params (DeltaSeconds :type Float%20%28single-precision%29)))

(fn ConstructionScript
  (bind _splinearray (Variables|Default|GetSplinearray))
  (Utilities|Array|Clear (Variables|Default|GetArrayPoints))
  (Spline|SetClosedLoop (Variables|Default|GetClosedLoop))
  (Variables|Default|SetSplineLastIndex (Class|SplineComponent|GetNumSplinePoints))
  (Variables|Default|SetSplineLastIndex (- (Variables|Default|GetSplineLastIndex) (Math|Integer|SelectInt 2 1 (Variables|Default|GetClosedLoop))))
  (Utilities|FlowControl|Sequence
    (:then_0
      (Math|Integer|CompareInt (+ (Variables|Default|GetSplineLastIndex) 1) (Utilities|Array|Length (Variables|Default|GetSplinearray)) :!label _label
        (:>
          (Utilities|Array|Add (Variables|Default|GetSplinearray) (Utilities|Struct|MakeSplinePathStructure false 0.8 false 0.0 false 1.0))
          (goto _label))
        (:<
          (Utilities|Array|RemoveIndex _splinearray (Utilities|Array|LastIndex _splinearray))
          (goto _label))))
    (:then_1
      (for _index (range 0 (Variables|Default|GetSplineLastIndex))
        (Utilities|Array|Add (Variables|Default|GetArrayPoints) (Math|Conversions|ToTransform(Vector) (Class|SplineComponent|GetWorldLocationatSplinePoint _index)))))
    (:then_2
      (if (Variables|Default|GetDrawNumbers)
        (for _index_2 (range 0 (Variables|Default|GetSplineLastIndex)) ; Run a loop for 0 to the number of the last spline point
          (Variables|Default|SetCurrentTrackNumber (Utilities|String|ToString(Integer) _index_2))
          (bind _returnvalue (AddComponent|AddTextRenderComponent false (Math|Transform|MakeTransform (Math|Vector|MakeVector (.X (Math|Vector|BreakVector (.LocalLocation (Class|SplineComponent|GetLocalLocationandTangentatSplinePoint (Variables|Default|GetSpline) _index_2)))) (.Y (Math|Vector|BreakVector (.LocalLocation (Class|SplineComponent|GetLocalLocationandTangentatSplinePoint (Variables|Default|GetSpline) _index_2)))) (+ (.Z (Math|Vector|BreakVector (.LocalLocation (Class|SplineComponent|GetLocalLocationandTangentatSplinePoint (Variables|Default|GetSpline) _index_2)))) 5e+01)) (Math|Conversions|RotationFromXVector (* (.LocalTangent (Class|SplineComponent|GetLocalLocationandTangentatSplinePoint (Variables|Default|GetSpline) _index_2)) -1.0))))) ; Creates a visible piece of text over the track point.
          (Rendering|Components|TextRender|SetText _returnvalue (Variables|Default|GetCurrentTrackNumber)))))))

(fn ReturnBackConnection
  (return (Variables|Default|GetBackConnection)))

(fn ReturnForwardConnection
  (return (Variables|Default|GetFowardConnection)))

(fn ReturnTransform
  (return (Variables|Default|GetArrayPoints)))

(fn SetPointVar
  (return (Variables|Default|GetPointvars) (Variables|Default|GetSplinearray)))