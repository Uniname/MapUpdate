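; Elliptical path actor that lays out a full or partial ellipse of goal-point transforms, apparently for the sedan to follow.
; The construction script spaces points by angle using stretch, rotation and step count, adding a mesh at each and optional numbered text labels.
; It resizes a per-point steering-suggestion array to match the points.
; Getter functions expose the transforms, forward and back connections, and steering suggestions.
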(event EventActorBeginOverlap
  (params (OtherActor :type Actor%20Object%20Reference)))

(event EventTick
  (params (DeltaSeconds :type Float%20%28single-precision%29)))

(event EventBeginPlay)

(fn ConstructionScript
  (bind _splinearray (Variables|Default|GetSplinearray))
  (Variables|Default|SetDegrees (Math|Float|Clamp(Float) (Variables|Default|GetDegrees) 0.0 3.6e+02))
  (Variables|Default|SetRotate (Math|Float|Clamp(Float) (Variables|Default|GetRotate) 0.0 3.6e+02))
  (Utilities|Array|Clear (Variables|Default|GetGoalTargets))
  (Variables|Default|SetStretchX (Variables|Default|GetStretchX))
  (Variables|Default|SetStretchY (Variables|Default|GetStretchY))
  (bind _output_get (Variables|Default|SetNumberofSteps (Variables|Default|GetNumberofSteps)))
  (Variables|Default|SetDegreeSteps (/ (Variables|Default|GetDegrees) (Math|Conversions|ToFloat(Integer) _output_get)))
  (for _index (range 0 (- (Variables|Default|GetNumberofSteps) 1))
    (Variables|Default|SetCurrentDegree (* _index (Variables|Default|GetDegreeSteps)))
    (Utilities|Array|Add (Variables|Default|GetGoalTargets) (Math|Conversions|ToTransform(Vector) (+ (Math|Vector|MakeVector (* (Math|Trig|Cos(Degrees) (+ (Variables|Default|GetCurrentDegree) (Variables|Default|GetRotate))) (Variables|Default|GetStretchX)) (* (Math|Trig|Sin(Degrees) (+ (Variables|Default|GetCurrentDegree) (Variables|Default|GetRotate))) (Variables|Default|GetStretchY)) 0.0) (Transformation|GetWorldLocation (Variables|Default|GetScene)))))
    (bind _returnvalue (AddComponent|AddStaticMeshComponent false (Math|Conversions|ToTransform(Vector) (Math|Vector|MakeVector (* (Math|Trig|Cos(Degrees) (+ (Variables|Default|GetCurrentDegree) (Variables|Default|GetRotate))) (Variables|Default|GetStretchX)) (* (Math|Trig|Sin(Degrees) (+ (Variables|Default|GetCurrentDegree) (Variables|Default|GetRotate))) (Variables|Default|GetStretchY)) 0.0))))
    (Components|StaticMesh|SetStaticMesh _returnvalue (Variables|Default|GetConstructedMesh)))
  (Utilities|FlowControl|Sequence
    (:then_0
      (Utilities|Array|Add (Variables|Default|GetSplinearray) (Utilities|Struct|MakeSplinePathStructure false 0.8 false 0.0 false 1.0) :!label _label)
      (Math|Integer|CompareInt (Utilities|Array|Length (Variables|Default|GetGoalTargets)) (Utilities|Array|Length (Variables|Default|GetSplinearray)) :!label _label_2
        (:>
          (goto _label))
        (:<
          (Utilities|Array|RemoveIndex _splinearray (Utilities|Array|LastIndex _splinearray))
          (goto _label_2))))
    (:then_1
      (if (Variables|Default|GetDrawNumbers)
        (for (_ _array_index) (Variables|Default|GetGoalTargets)
          (Variables|Default|SetCurrentTrackNumber (Utilities|String|ToString(Integer) _array_index))
          (bind _returnvalue_2 (AddComponent|AddTextRenderComponent false (Math|Transform|MakeTransform (- (Math|Vector|MakeVector (.X (Math|Vector|BreakVector (.Location (Math|Transform|BreakTransform (Utilities|Array|Get(acopy) (Variables|Default|GetGoalTargets) _array_index))))) (.Y (Math|Vector|BreakVector (.Location (Math|Transform|BreakTransform (Utilities|Array|Get(acopy) (Variables|Default|GetGoalTargets) _array_index))))) (+ (.Z (Math|Vector|BreakVector (.Location (Math|Transform|BreakTransform (Utilities|Array|Get(acopy) (Variables|Default|GetGoalTargets) _array_index))))) 5e+01)) (Transformation|GetWorldLocation (Variables|Default|GetScene))) (Math|Rotator|FindLookatRotation (Math|Vector|MakeVector (.X (Math|Vector|BreakVector (.Location (Math|Transform|BreakTransform (Utilities|Array|Get(acopy) (Variables|Default|GetGoalTargets) _array_index))))) (.Y (Math|Vector|BreakVector (.Location (Math|Transform|BreakTransform (Utilities|Array|Get(acopy) (Variables|Default|GetGoalTargets) _array_index))))) (+ (.Z (Math|Vector|BreakVector (.Location (Math|Transform|BreakTransform (Utilities|Array|Get(acopy) (Variables|Default|GetGoalTargets) _array_index))))) 5e+01)) (Math|Vector|MakeVector 0.0 0.0 0.0))))) ; Creates a visible piece of text over the track point.
          (Rendering|Components|TextRender|SetText _returnvalue_2 (Variables|Default|GetCurrentTrackNumber)))))))

(fn FunctionFindX
  (params (BValue :type Float%20%28single-precision%29 :default 0.0) (AValue :type Float%20%28single-precision%29 :default 0.0) (YSquared :type Float%20%28single-precision%29 :default 0.0))
  (return (Math|Float|Sqrt (/ (- (* BValue AValue) (* AValue (Math|Float|Square YSquared))) BValue))))

(fn ReturnBackConnection
  (return (Variables|Default|GetBackConnection)))

(fn ReturnForwardConnection
  (return (Variables|Default|GetForwardConnection)))

(fn ReturnTransform
  (return (Variables|Default|GetGoalTargets)))

(fn SetPointVar
  (return (Variables|Default|GetPointSuggestions) (Variables|Default|GetSplinearray)))