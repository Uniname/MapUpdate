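; Controller for the sedan vehicle that finds the start actor and kicks off its pawn's startup with the game mode's direction setting.
; One second after BeginPlay, a timer searches actors implementing the Return interface for the one tagged "First" and caches it as StartActor.
; It then sends StartUPWorkMessage to the controlled pawn with the VehicleGameMode's Reversed value.
; REturnStartActor exposes the cached actor.
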(event Custom|Break
  (Utilities|Array|ForEachLoopwithBreak (stale Custom|Wait _outactors)) ; enters at Break
)

(event Custom|Wait
  (bind _outactors (Actor|GetAllActorswithInterface "/Game/Blueprints/SedanBlueprint/Return.Return_C"))
  (bind _array_element (Utilities|Array|ForEachLoopwithBreak _outactors)
    (:LoopBody
      (if (Actor|ActorHasTag _array_element "First")
        (Variables|Default|SetStartActor _array_element)
        (bind _asvehicle_game_mode (Utilities|Casting|CastToVehicleGameMode (Game|GetGameMode)))
        (Class|StartgameINterface|StartUPWork(Message) (Pawn|GetControlledPawn) (Variables|/Game/Blueprints/SedanBlueprint/VehicleGameMode.VehicleGameMode_C|GetReversed _asvehicle_game_mode))
        (CallFunction|Break)))))

(event EventBeginPlay
  (Utilities|Time|SetTimerbyEvent (delegate Custom|Wait) 1.0))

(event EventTick
  (params (DeltaSeconds :type Float%20%28single-precision%29)))

(fn ConstructionScript)

(fn REturnStartActor
  (return (Variables|Default|GetStartActor)))