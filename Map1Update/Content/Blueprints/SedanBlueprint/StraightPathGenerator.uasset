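; Straight path segment actor that lays out evenly spaced goal transforms, with per-point steering suggestions, apparently for the sedan to follow.
; The construction script steps from the actor toward a flattened EndLocation, facing each point at the end and offsetting by world location only.
; It resizes the steering array to match and can spawn preview meshes and index labels.
; Getter functions expose the targets, suggestions and forward/back connections.
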(event EventActorBeginOverlap
  (params (OtherActor :type Actor%20Object%20Reference)))

(event EventTick
  (params (DeltaSeconds :type Float%20%28single-precision%29)))

(event EventBeginPlay)

(fn ConstructionScript
  (bind _endlocation (Variables|Default|GetEndLocation))
  (bind _splinearray (Variables|Default|GetSplinearray))
  (bind _returnvalue (* _endlocation "1.000000,1.000000,0.000000"))
  (Variables|Default|SetDegrees (Math|Float|Clamp(Float) (Variables|Default|GetDegrees) 0.0 3.6e+02))
  (Variables|Default|SetNumberofSteps (Math|Integer|Clamp(Integer) (Variables|Default|GetNumberofSteps) 0 40))
  (Utilities|Array|Clear (Variables|Default|GetGoalTargets))
  (for _index (range 0 (- (Variables|Default|GetNumberofSteps) 0))
    (Utilities|Array|Add (Variables|Default|GetGoalTargets) (Math|Transform|MakeTransform (+ (.Location (Math|Transform|BreakTransform (Math|Transform|MakeTransform (Math|Vector|MakeVector (* _index (.X (Math|Vector|BreakVector (/ _returnvalue (Math|Conversions|ToFloat(Integer) (Variables|Default|GetNumberofSteps)))))) (* _index (.Y (Math|Vector|BreakVector (/ _returnvalue (Math|Conversions|ToFloat(Integer) (Variables|Default|GetNumberofSteps)))))) 0.0) (Math|Rotator|FindLookatRotation (Math|Vector|MakeVector (* _index (.X (Math|Vector|BreakVector (/ _returnvalue (Math|Conversions|ToFloat(Integer) (Variables|Default|GetNumberofSteps)))))) (* _index (.Y (Math|Vector|BreakVector (/ _returnvalue (Math|Conversions|ToFloat(Integer) (Variables|Default|GetNumberofSteps)))))) 0.0) _returnvalue)))) (Transformation|GetWorldLocation)) (.Rotation (Math|Transform|BreakTransform (Math|Transform|MakeTransform (Math|Vector|MakeVector (* _index (.X (Math|Vector|BreakVector (/ _returnvalue (Math|Conversions|ToFloat(Integer) (Variables|Default|GetNumberofSteps)))))) (* _index (.Y (Math|Vector|BreakVector (/ _returnvalue (Math|Conversions|ToFloat(Integer) (Variables|Default|GetNumberofSteps)))))) 0.0) (Math|Rotator|FindLookatRotation (Math|Vector|MakeVector (* _index (.X (Math|Vector|BreakVector (/ _returnvalue (Math|Conversions|ToFloat(Integer) (Variables|Default|GetNumberofSteps)))))) (* _index (.Y (Math|Vector|BreakVector (/ _returnvalue (Math|Conversions|ToFloat(Integer) (Variables|Default|GetNumberofSteps)))))) 0.0) _returnvalue))))))
    (if (Variables|Default|GetShowMesh)
      (bind _returnvalue_2 (AddComponent|AddStaticMeshComponent false (Math|Transform|MakeTransform (Math|Vector|MakeVector (* _index (.X (Math|Vector|BreakVector (/ _returnvalue (Math|Conversions|ToFloat(Integer) (Variables|Default|GetNumberofSteps)))))) (* _index (.Y (Math|Vector|BreakVector (/ _returnvalue (Math|Conversions|ToFloat(Integer) (Variables|Default|GetNumberofSteps)))))) 0.0) (Math|Rotator|FindLookatRotation (Math|Vector|MakeVector (* _index (.X (Math|Vector|BreakVector (/ _returnvalue (Math|Conversions|ToFloat(Integer) (Variables|Default|GetNumberofSteps)))))) (* _index (.Y (Math|Vector|BreakVector (/ _returnvalue (Math|Conversions|ToFloat(Integer) (Variables|Default|GetNumberofSteps)))))) 0.0) _returnvalue))))
      (Components|StaticMesh|SetStaticMesh _returnvalue_2 (Variables|Default|GetConstructedMesh))))
  (Utilities|FlowControl|Sequence
    (:then_0
      (Utilities|Array|Add (Variables|Default|GetSplinearray) (Utilities|Struct|MakeSplinePathStructure false 0.8 false 0.0 false 1.0) :!label _label)
      (Math|Integer|CompareInt (Utilities|Array|Length (Variables|Default|GetGoalTargets)) (Utilities|Array|Length (Variables|Default|GetSplinearray)) :!label _label_2
        (:>
          (goto _label))
        (:<
          (Utilities|Array|RemoveIndex _splinearray (Utilities|Array|LastIndex _splinearray))
          (goto _label_2))))
    (:then_1
      (if (Variables|Default|GetDrawNumbers)
        (for (_ _array_index) (Variables|Default|GetGoalTargets)
          (Variables|Default|SetCurrentTrackNumber (Utilities|String|ToString(Integer) _array_index))
          (bind _returnvalue_3 (AddComponent|AddTextRenderComponent false (Math|Transform|MakeTransform (- (Math|Vector|MakeVector (.X (Math|Vector|BreakVector (.Location (Math|Transform|BreakTransform (Utilities|Array|Get(acopy) (Variables|Default|GetGoalTargets) _array_index))))) (.Y (Math|Vector|BreakVector (.Location (Math|Transform|BreakTransform (Utilities|Array|Get(acopy) (Variables|Default|GetGoalTargets) _array_index))))) (+ (.Z (Math|Vector|BreakVector (.Location (Math|Transform|BreakTransform (Utilities|Array|Get(acopy) (Variables|Default|GetGoalTargets) _array_index))))) 5e+01)) (Transformation|GetWorldLocation (Variables|Default|GetScene))) (Math|Rotator|FindLookatRotation (Math|Vector|MakeVector (.X (Math|Vector|BreakVector (.Location (Math|Transform|BreakTransform (Utilities|Array|Get(acopy) (Variables|Default|GetGoalTargets) _array_index))))) (.Y (Math|Vector|BreakVector (.Location (Math|Transform|BreakTransform (Utilities|Array|Get(acopy) (Variables|Default|GetGoalTargets) _array_index))))) (+ (.Z (Math|Vector|BreakVector (.Location (Math|Transform|BreakTransform (Utilities|Array|Get(acopy) (Variables|Default|GetGoalTargets) _array_index))))) 5e+01)) (Math|Vector|MakeVector 0.0 0.0 0.0))))) ; Creates a visible piece of text over the track point.
          (Rendering|Components|TextRender|SetText _returnvalue_3 (Variables|Default|GetCurrentTrackNumber)))))))

(fn ReturnBackConnection
  (return (Variables|Default|GetBackConnection)))

(fn ReturnForwardConnection
  (return (Variables|Default|GetForwardConnection)))

(fn ReturnTransform
  (return (Variables|Default|GetGoalTargets)))

(fn SetPointVar
  (return (Variables|Default|GetPointNON) (Variables|Default|GetSplinearray)))